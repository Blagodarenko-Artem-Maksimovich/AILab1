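; Labyrinth bot that drives itself forward and steers away from obstacles, with all logic in Tick.
; Each frame it makes a swept move along its forward vector, then fires two debug-drawn Visibility traces angled ahead-right and ahead-left.
; Each clear trace nudges yaw toward that side, so two clear sides cancel out and two blocked sides give no turn.
; Movement and turning are fixed per-frame steps, independent of delta time.
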(event `self.ReceiveTick`
  (params (DeltaSeconds :type "Float (single-precision)"))
  (bind _returnvalue (`self.K2_GetActorLocation`))
  (bind _returnvalue_2 (`self.K2_GetActorLocation`))
  (`self.K2_SetActorLocation` (+ (`self.K2_GetActorLocation`) (* (`self.GetActorForwardVector`) 5.0)) true)
  (bind (_outhit _returnvalue_3) (`KismetSystemLibrary.LineTraceSingle` :`Start` _returnvalue_2 :`End` (+ _returnvalue_2 (* (+ (`self.GetActorForwardVector`) (/ (`self.GetActorRightVector`) 2.0)) 400.0)) :`TraceChannel` "TraceTypeQuery1" :`DrawDebugType` "ForDuration" :`DrawTime` 0.1))
  (if (not _returnvalue_3)
    (`self.K2_SetActorRotation` (`KismetMathLibrary.ComposeRotators` (`self.K2_GetActorRotation`) (struct :`Yaw` 2.0))))
  (bind (_outhit_2 _returnvalue_4) (`KismetSystemLibrary.LineTraceSingle` :`Start` _returnvalue :`End` (+ _returnvalue (* (- (`self.GetActorForwardVector`) (/ (`self.GetActorRightVector`) 2.0)) 400.0)) :`TraceChannel` "TraceTypeQuery1" :`DrawDebugType` "ForDuration" :`DrawTime` 0.1))
  (if (not _returnvalue_4)
    (`self.K2_SetActorRotation` (`KismetMathLibrary.ComposeRotators` (`self.K2_GetActorRotation`) (struct :`Yaw` -2.0)))))

(fn `UserConstructionScript`)